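; BP_Door is an interactive door item that swings open and closed, and can be locked behind required inventory items.
; Using it while locked opens a WB_DoorTask widget with those items, otherwise a timeline rotates the mesh around its starting yaw.
; CheckInventory sets Locked from each item lookup in turn, so the last one decides, then on success removes the items and opens the door.
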(event `self.ReceiveBeginPlay`
  (bind (_returnvalue_roll _returnvalue_pitch _returnvalue_yaw) (`KismetMathLibrary.BreakRotator` (`self.K2_GetActorRotation`)))
  (bind _output_get (set `self.StartRotate` _returnvalue_yaw))
  (if (`self.Door Open`)
    (`SceneComponent.K2_SetRelativeRotation` (`self.MeshItem`) (`KismetMathLibrary.MakeRotator` 0.0 0.0 (+ _output_get -90.0)) false false)))

(event `Open Door`
  (if (`self.Door Open`)
    (bind (_direction _newtrack_0) (`Timeline|Timeline_OpenDoor` :!via `ReverseFromEnd` :!label _label)
      (:`Update`
        (`SceneComponent.K2_SetRelativeRotation` (`self.MeshItem`) (`KismetMathLibrary.MakeRotator` 0.0 0.0 (+ (`self.StartRotate`) _newtrack_0)) false false))
      (:`Finished`
        (set `self.Door Open` (< _newtrack_0 0.0))))
    (else
      (goto _label))))

(fn `CheckInventory`
  (params (TargetPlayer :type "/Game/TopAcademy/Blueprints/Objects/Player/BP_MainPlayer Object Reference"))
  (returns (Opened :type Boolean))
  (locals (NewLocalVar :type Integer))
  (bind _inventory (`/Game/TopAcademy/Blueprints/Objects/Player/BP_MainPlayer.Inventory` TargetPlayer))
  (for _array_element (`self.Items`)
    (bind _index (`/Game/TopAcademy/Inventory/BPC_Inventory.FindItem` _inventory _array_element))
    (set `self.Locked` (not (>= _index 0))))
  (if (`self.Locked`)
    (return false)
    (else
      (for _array_element_2 (`self.Items`)
        (bind _index_2 (`/Game/TopAcademy/Inventory/BPC_Inventory.FindItem` _inventory _array_element_2))
        (`/Game/TopAcademy/Inventory/BPC_Inventory.RemoveItem` _inventory _index_2))
      (`self.Open Door`)
      (return true))))

(fn `ScanItemHand`
  (params (Player :type "/Game/TopAcademy/Blueprints/Objects/Player/BP_MainPlayer Object Reference"))
  (returns (Flag :type Boolean))
  (`/Game/TopAcademy/Blueprints/Objects/Player/BP_MainPlayer.ShowCloseHand` Player true)
  (return true))

(fn `UseItem`
  (params (Player :type "/Game/TopAcademy/Blueprints/Objects/Player/BP_MainPlayer Object Reference"))
  (if (`self.Locked`)
    (bind _returnvalue (`|CreateWidget` "/Game/TopAcademy/Hud/Door/WB_DoorTask.WB_DoorTask_C"))
    (`UserWidget.AddToViewport` _returnvalue 0)
    (`/Game/TopAcademy/Hud/Door/WB_DoorTask.Init Tasks` _returnvalue (`self.Items`) Player self)
    (else
      (`self.Open Door`)))
  (return))

(fn `UserConstructionScript`
  (`parent.UserConstructionScript`))