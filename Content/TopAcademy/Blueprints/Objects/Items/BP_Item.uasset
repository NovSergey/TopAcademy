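; BP_Item is a world item actor that players can pick up into their inventory.
; An Info struct supplies the static mesh set on MeshItem through SetNewMesh.
; UseItem destroys the actor and adds Info to the player's inventory, while ScanItemHand shows the player's close-hand indicator.
; PickupItem is an empty stub.
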(event `SetNewMesh`
  (bind (_info_id _info_name _info_icon _info_mesh) (break `/Game/TopAcademy/Inventory/S_ItemStruct` (`self.Info`)))
  (`StaticMeshComponent.SetStaticMesh` (`self.MeshItem`) _info_mesh))

(event `/Game/TopAcademy/Blueprints/Interfaces/I_PickableItem.UseItem`
  (params (Player :type "/Game/TopAcademy/Blueprints/Objects/Player/BP_MainPlayer Object Reference"))
  (`self.K2_DestroyActor`)
  (`/Game/TopAcademy/Inventory/BPC_Inventory.AddItemToInventory` (`/Game/TopAcademy/Blueprints/Objects/Player/BP_MainPlayer.Inventory` Player) (`self.Info`)))

(fn `PickupItem`
  (return))

(fn `ScanItemHand`
  (params (Player :type "/Game/TopAcademy/Blueprints/Objects/Player/BP_MainPlayer Object Reference"))
  (returns (Flag :type Boolean))
  (`/Game/TopAcademy/Blueprints/Objects/Player/BP_MainPlayer.ShowCloseHand` Player true)
  (return true))

(fn `UserConstructionScript`
  (`parent.UserConstructionScript`))