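; BP_SpawnerItems is a spawner actor that creates items at random locations inside its box volume.
; Its SpawnActor function picks a random point within the scaled BoxSpawner extent around the actor and spawns SpawnerClass there.
; If the result is a BP_Item, it copies the passed ItemMesh into the item's Info and calls SetNewMesh.
; BeginPlay and the construction script are empty, so nothing spawns until SpawnActor is called.
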(event `self.ReceiveBeginPlay`)

(fn `Spawn Actor`
  (params (ItemMesh :type "/Game/TopAcademy/Inventory/S_ItemStruct Structure"))
  (bind _output_get (set `self.RandomLocation` (`KismetMathLibrary.RandomPointInBoundingBox` (`self.K2_GetActorLocation`) (`BoxComponent.GetScaledBoxExtent` (`self.BoxSpawner`)))))
  (bind _returnvalue (`|SpawnActorFromClass` (`self.SpawnerClass`) (`KismetMathLibrary.Conv_VectorToTransform` _output_get) "Undefined" "MultiplyWithRoot" null null))
  (bind _asbp_item (cast `/Game/TopAcademy/Blueprints/Objects/Items/BP_Item` _returnvalue))
  (set `/Game/TopAcademy/Blueprints/Objects/Items/BP_Item.Info` ItemMesh _asbp_item)
  (`/Game/TopAcademy/Blueprints/Objects/Items/BP_Item.SetNewMesh` _asbp_item))

(fn `UserConstructionScript`)