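; Player character for touch devices, with joystick movement, swipe camera look, item interaction and an inventory.
; A looping timer line-traces from the camera and messages the hit actor, hiding the HUD hand when nothing responds.
; UseHand sends a use message to that actor, while wrapper functions forward item changes to the Inventory component.
; Touch press opens a gate that Tick polls, turning finger movement beyond a threshold into yaw and pitch.
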(event `ShowOpenInventory`
  (bind _foundwidgets (`WidgetBlueprintLibrary.GetAllWidgetsOfClass` "/Game/TopAcademy/Hud/Inventory/WB_Inventory.WB_Inventory_C"))
  (if (== (`KismetArrayLibrary.Array_Length` _foundwidgets) 0)
    (bind _returnvalue (`|CreateWidget` "/Game/TopAcademy/Hud/Inventory/WB_Inventory.WB_Inventory_C"))
    (`UserWidget.AddToViewport` _returnvalue 0)
    (`/Game/TopAcademy/Hud/Inventory/WB_Inventory.Init Inventory` _returnvalue (`/Game/TopAcademy/Inventory/BPC_Inventory.Inventory` (`self.Inventory`)))
    (else
      (`Widget.RemoveFromParent` _foundwidgets))))

(event `ShowCloseHand`
  (params (Flag :type Boolean))
  (bind _foundwidgets (`WidgetBlueprintLibrary.GetAllWidgetsOfClass` "/Game/TopAcademy/Hud/WB_Hud.WB_Hud_C"))
  (for _array_element _foundwidgets
    (bind _aswb_hud (cast `/Game/TopAcademy/Hud/WB_Hud` _array_element))
    (if Flag
      (bind _usehand (`/Game/TopAcademy/Hud/WB_Hud.UseHand` _aswb_hud))
      (`Widget.SetVisibility` _usehand "Visible")
      (else
        (`Widget.SetVisibility` _usehand "Hidden")))))

(event `self.ReceiveBeginPlay`
  (`PlayerController.ActivateTouchInterface` (`GameplayStatics.GetPlayerController` 0) "/Game/TopAcademy/Hud/LeftVirtualJoystickOnly.LeftVirtualJoystickOnly")
  (`KismetSystemLibrary.K2_SetTimer` null "ScanItem" 0.25 true)
  (bind _returnvalue (`|CreateWidget` "/Game/TopAcademy/Hud/WB_Hud.WB_Hud_C"))
  (`UserWidget.AddToViewport` _returnvalue 0))

(event `InputAxis|MoveForwardBackward`
  (params (AxisValue :type "Float (single-precision)"))
  ;[1 1 1] Character Movement
  (`self.AddMovementInput` (`KismetMathLibrary.GetForwardVector` (`KismetMathLibrary.MakeRotator` 0.0 0.0 (.yaw (`self.GetControlRotation`)))) AxisValue))

(event `InputAxis|MoveLeftRight`
  (params (AxisValue :type "Float (single-precision)"))
  ;[1 1 1] Character Movement
  (`self.AddMovementInput` (`KismetMathLibrary.GetRightVector` (`KismetMathLibrary.MakeRotator` 0.0 0.0 (.yaw (`self.GetControlRotation`)))) AxisValue))

(event `Touch`
  ;[1 1 1] Comment
  (`/Engine/EditorBlueprintResources/StandardMacros.Gate` true :!label _label
    (:`Exit`
      (bind (_locationx _locationy) (`PlayerController.GetInputTouchState` (`GameplayStatics.GetPlayerController` 0) (stale `InputTouch` FingerIndex)))
      (bind _returnvalue (`KismetMathLibrary.MakeVector2D` _locationx _locationy))
      (if (>= (`KismetMathLibrary.VSize2D` (- _returnvalue (stale `InputTouch` _output_get))) (`self.Swipethreshold`))
        (set `self.Startloc` (100000.0 100000.0))
        (bind (_returnvalue_x _returnvalue_y) (`KismetMathLibrary.BreakVector2D` (* (- _returnvalue (`self.Priorloc`)) (`self.Swipespeed`))))
        (`self.AddControllerYawInput` _returnvalue_x)
        (`self.AddControllerPitchInput` _returnvalue_y)
        (set `self.Priorloc` _returnvalue)))))

(event `InputTouch`
  (params (Location :type "Vector Structure") (FingerIndex :type "ETouchIndex Enum"))
  (bind (_locationx _locationy) (`PlayerController.GetInputTouchState` (`GameplayStatics.GetPlayerController` 0) FingerIndex))
  ;[1 1 1] Comment
  (:`Pressed`
    (bind _output_get (set `self.Startloc` (`KismetMathLibrary.MakeVector2D` _locationx _locationy)))
    (set `self.Priorloc` _output_get)
    (goto _label :!via `Open`)))

(event `self.ReceiveTick`
  (params (DeltaSeconds :type "Float (single-precision)"))
  (`self.Touch`))

(fn `AddItemToIventory`
  (params (Info :type "/Game/TopAcademy/Inventory/S_ItemStruct Structure"))
  (`/Game/TopAcademy/Inventory/BPC_Inventory.AddItemToInventory` (`self.Inventory`) Info))

(fn `GetInventory`
  (returns (Inventory :type "Array of /Game/TopAcademy/Inventory/S_ItemStruct Structure"))
  (return (`/Game/TopAcademy/Inventory/BPC_Inventory.Inventory` (`self.Inventory`))))

(fn `RemoveItemFromInventory`
  (params (Item :type "/Game/TopAcademy/Inventory/S_ItemStruct Structure"))
  (`/Game/TopAcademy/Inventory/BPC_Inventory.RemoveItemFromInventory` (`self.Inventory`) Item))

(fn `ScanItem`
  (bind _camera (`self.Camera`))
  (bind _returnvalue (`SceneComponent.K2_GetComponentLocation` _camera))
  (bind (_outhit _returnvalue_2) (`KismetSystemLibrary.LineTraceSingle` _returnvalue (+ _returnvalue (* (`KismetMathLibrary.GetForwardVector` (`SceneComponent.K2_GetComponentRotation` _camera)) 300.0)) "TraceTypeQuery1"))
  (if _returnvalue_2
    (set `self.Hit Actor` (`.HitActor` (`GameplayStatics.BreakHitResult` _outhit)))
    (bind _hit_actor (`self.Hit Actor`)
      (:`then`
        (bind _flag (message `/Game/TopAcademy/Blueprints/Interfaces/I_PickableItem.ScanItemHand` _hit_actor self))
        (if (not _flag)
          (`self.ShowCloseHand` false :!label _label)))
      (:`else`))
    (else
      (goto _label))))

(fn `TryPickupItem`
  (params (Pickup :type "Actor Object Reference"))
  (message `/Game/TopAcademy/Blueprints/Interfaces/I_PickableItem.UseItem` Pickup self))

(fn `UseHand`
  (bind _hit_actor (`self.Hit Actor`)
    (:`then`
      (`self.TryPickupItem` _hit_actor))
    (:`else`)))

(fn `UserConstructionScript`)