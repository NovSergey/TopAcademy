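; Inventory component that stores items in an array and provides functions to add, find and remove them.
; AddItemToInventory appends an item without duplicate or capacity checks.
; FindItem scans the array for a matching Id and Name and returns its index, or -1 when absent.
; RemoveItem deletes the entry at a given index.
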(fn `AddItemToInventory`
  (params (Item :type "/Game/TopAcademy/Inventory/S_ItemStruct Structure"))
  (`KismetArrayLibrary.Array_Add` (`self.Inventory`) Item))

(fn `FindItem`
  (params (Item :type "/Game/TopAcademy/Inventory/S_ItemStruct Structure"))
  (returns (Index :type Integer))
  (for (_array_element _array_index) (`self.Inventory`)
    (if (and (== (break `/Game/TopAcademy/Inventory/S_ItemStruct` _array_element) Item_Id_21_A2EB60BB499BDA9E0C4FD3A642F97A1D) (`KismetTextLibrary.EqualEqual_TextText` (`.Name_22_8959422647BF136B10A582B99BF638C8` (break `/Game/TopAcademy/Inventory/S_ItemStruct` _array_element)) Item_Name_22_8959422647BF136B10A582B99BF638C8))
      (return _array_index)))
  (return -1))

(fn `RemoveItem`
  (params (Index :type Integer))
  (`KismetArrayLibrary.Array_Remove` (`self.Inventory`) Index))